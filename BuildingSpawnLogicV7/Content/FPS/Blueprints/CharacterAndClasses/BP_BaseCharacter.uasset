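; BP_BaseCharacter is the base Blueprint character for the FPS, providing replicated weapon and death state for child classes.
; A server-only pawn death event sets the Dead flag, whose RepNotify calls the overridable OnDeadRep hook, meant for ragdoll, and fires CallOnDeath.
; The current weapon RepNotify forwards to OnCurrentWeaponChanged, which is left empty alongside OnEquippedWeaponChanged.
; A delayed respawn request through BP_Base_GM is present but disconnected.
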(event `OnCurrentWeaponChanged`)

(event `OnEquippedWeaponChanged`)

(event `OnPawnDead`
  ;[1 1 1] Server Only
  (set `self.bDead` true))

(fn `OnDeadRep`)

(fn `OnRep_bDead`
  (`self.OnDeadRep`) ; To activate Ragdoll if needed, override on child classes
  (if (`self.bDead`)
    (`self.OnDeath`)))

(fn `OnRep_CurrentWeapon`
  (`self.OnCurrentWeaponChanged`))

(fn `UserConstructionScript`)
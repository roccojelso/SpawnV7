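; Game instance for the Influence Spawn System demo that manages LAN multiplayer sessions through create, join and destroy events.
; Creating hosts a LAN session with the given player limit and opens the lobby level as a listen server.
; Joining stores the session's player limit, and destroying returns to the main menu level.
; Successful operations update flags tracking whether the local player created or joined a lobby.
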(event `CreateSession`
  (params (`Max Players Count` :type Integer))
  ;[1 1 1] CREATE SESSION
  (bind _output_get (set `self.Max Plr Count` `Max Players Count`))
  (`CreateSessionCallbackProxy.CreateSession` (`GameplayStatics.GetPlayerController` 0) _output_get true
    (:`OnSuccess`
      (set `self.ControllerCreatedLobby?` true)
      (`GameplayStatics.OpenLevel` "ISSDemoLobbyMenu" true "listen"))))

(event `JoinSession`
  (params (SearchResult :type "BlueprintSessionResult Structure (by ref)"))
  ;[1 1 1] JOIN TO SESSION
  (set `self.Max Plr Count` (`FindSessionsCallbackProxy.GetMaxPlayers` SearchResult))
  (`JoinSessionCallbackProxy.JoinSession` (`GameplayStatics.GetPlayerController` 0) SearchResult
    (:`OnSuccess`
      (set `self.ControllerJoinedLobby?` true))))

(event `DestroySession`
  ;[1 1 1] DESTROY SESSION
  (`DestroySessionCallbackProxy.DestroySession` (`GameplayStatics.GetPlayerController` 0)
    (:`OnSuccess`
      (set `self.ControllerCreatedLobby?` false)
      (set `self.ControllerJoinedLobby?` false)
      (`GameplayStatics.OpenLevel` "ISSDemoMainMenu" true "listen"))))
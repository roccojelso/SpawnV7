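; Test domination point for the Influence Spawn System that simulates being captured by alternating teams.
; On Tick, a Delay and FlipFlop switch the mesh between blue for Team 2 and red for Team 1 every ten seconds.
; On standalone or server, each switch sets the team ID component and restarts both game-mode influence components (positive to owner, negative to enemy), which BeginPlay initially stops.
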(event `self.ReceiveBeginPlay`
  ;[1 1 1] EVENT BEGIN PLAY
  ;;[1 1 1] Check Standalone or Server Side
  (if (`KismetSystemLibrary.IsStandalone`)
    ;;[1 1 1] Stop BP_ISS_GameModeInfluence_PosToOwner
    (`/Game/InfluenceSpawnSystem/Blueprints/InfluenceSpawnSystem/Influences/SP_BaseInfluence.StopInfluence` (`self.BP_ISS_GameModeInfluence_PosToOwner`) :!label _label)
    ;;[1 1 1] Stop BP_ISS_GameModeInfluence_NegToEnemy
    (`/Game/InfluenceSpawnSystem/Blueprints/InfluenceSpawnSystem/Influences/SP_BaseInfluence.StopInfluence` (`self.BP_ISS_GameModeInfluence_NegToEnemy`))
    (elif (`KismetSystemLibrary.IsServer`)
      (goto _label))))

(event `self.ReceiveTick`
  (params (DeltaSeconds :type "Float (single-precision)"))
  ;[1 1 1] EVENT TICK
  ;;[1 1 1] Delay with flip Flop for simulation capture point of different team
  (`KismetSystemLibrary.Delay` 10.0)
  (`/Engine/EditorBlueprintResources/StandardMacros.FlipFlop`
    (:`A`
      ;;[1 1 1] Team 2 Captrure Point
      ;;;[1 1 1] Set Materials (Blue) for team 2
      (`PrimitiveComponent.SetMaterial` (`self.mesh`) 0 "/Game/InfluenceSpawnSystem/Materials/M_TestGameObjBlue.M_TestGameObjBlue")
      ;;;[1 1 1] Check Standalone or Server Side
      (if (`KismetSystemLibrary.IsStandalone`)
        ;;;[1 1 1] Set TeamID - Team 2
        (`/Game/InfluenceSpawnSystem/Blueprints/InfluenceSpawnSystem/SP_TeamID.ServerInitializeTeam` (`self.BP_ISS_TeamID`) "NewEnumerator2" :!label _label_2)
        ;;[1 1 1] Stop & Restart BP_ISS_GameModeInfluence_PosToOwner
        (`/Game/InfluenceSpawnSystem/Blueprints/InfluenceSpawnSystem/Influences/SP_BaseInfluence.StopInfluence` (`self.BP_ISS_GameModeInfluence_PosToOwner`) :!label _label_3)
        (`/Game/InfluenceSpawnSystem/Blueprints/InfluenceSpawnSystem/Influences/SP_BaseInfluence.ReStartInfluence` (`self.BP_ISS_GameModeInfluence_PosToOwner`))
        ;;[1 1 1] Stop & Restart BP_ISS_GameModeInfluence_NegToEnemy
        (`/Game/InfluenceSpawnSystem/Blueprints/InfluenceSpawnSystem/Influences/SP_BaseInfluence.StopInfluence` (`self.BP_ISS_GameModeInfluence_NegToEnemy`))
        (`/Game/InfluenceSpawnSystem/Blueprints/InfluenceSpawnSystem/Influences/SP_BaseInfluence.ReStartInfluence` (`self.BP_ISS_GameModeInfluence_NegToEnemy`))
        (elif (`KismetSystemLibrary.IsServer`)
          (goto _label_2))))
    (:`B`
      ;;[1 1 1] Team 1 Captrure Point
      ;;;[1 1 1] Set Materials (Red) for team 1
      (`PrimitiveComponent.SetMaterial` (`self.mesh`) 0 "/Game/InfluenceSpawnSystem/Materials/M_TestGameObjRed.M_TestGameObjRed")
      ;;;[1 1 1] Check Standalone or Server Side
      (if (`KismetSystemLibrary.IsStandalone`)
        ;;;[1 1 1] Set TeamID - Team 1
        (`/Game/InfluenceSpawnSystem/Blueprints/InfluenceSpawnSystem/SP_TeamID.ServerInitializeTeam` (`self.BP_ISS_TeamID`) "NewEnumerator1" :!label _label_4)
        (goto _label_3)
        (elif (`KismetSystemLibrary.IsServer`)
          (goto _label_4))))))

(fn `UserConstructionScript`)
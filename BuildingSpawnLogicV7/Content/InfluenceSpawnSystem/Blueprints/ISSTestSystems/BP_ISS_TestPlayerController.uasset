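; Test player controller for the Influence Spawn System that drives the controlled pawn and provides hooks for testing death and respawn.
; Axis inputs turn, look and move the pawn, using only control yaw so movement stays on the horizontal plane.
; The TestRespawn action calls ServerTestDeath on the test character.
; A separate RespawnPlayerCharacter event forwards respawn requests to the test game mode's CharacterRespawn.
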(event `InputAxis|Turn`
  (params (AxisValue :type "Float (single-precision)"))
  ;[1 1 1] TURN & LOOK UP
  (`/Engine/EditorBlueprintResources/StandardMacros.IsValid` (`self.K2_GetPawn`)
    (:`Is Valid`
      (`Pawn.AddControllerYawInput` (`self.K2_GetPawn`) AxisValue))))

(event `InputAxis|MoveForward`
  (params (AxisValue :type "Float (single-precision)"))
  ;[1 1 1] MOVEMENT FORWARD & BACK
  (`/Engine/EditorBlueprintResources/StandardMacros.IsValid` (`self.K2_GetPawn`)
    (:`Is Valid`
      (`Pawn.AddMovementInput` (`self.K2_GetPawn`) (`KismetMathLibrary.GetForwardVector` (`KismetMathLibrary.MakeRotator` 0.0 0.0 (.yaw (`Pawn.GetControlRotation` (`self.K2_GetPawn`))))) AxisValue false))))

(event `InputAxis|LookUp`
  (params (AxisValue :type "Float (single-precision)"))
  ;[1 1 1] TURN & LOOK UP
  (`/Engine/EditorBlueprintResources/StandardMacros.IsValid` (`self.K2_GetPawn`)
    (:`Is Valid`
      (`Pawn.AddControllerPitchInput` (`self.K2_GetPawn`) AxisValue))))

(event `InputAxis|MoveRight`
  (params (AxisValue :type "Float (single-precision)"))
  ;[1 1 1] MOVEMENT FORWARD & BACK
  (`/Engine/EditorBlueprintResources/StandardMacros.IsValid` (`self.K2_GetPawn`)
    (:`Is Valid`
      (`Pawn.AddMovementInput` (`self.K2_GetPawn`) (`KismetMathLibrary.GetRightVector` (`KismetMathLibrary.MakeRotator` 0.0 0.0 (.yaw (`Pawn.GetControlRotation` (`self.K2_GetPawn`))))) AxisValue false))))

(event `InputAction|TestRespawn`
  (params (Key :type "Key Structure"))
  ;[1 1 1] TEST RESPAWN
  (:`Pressed`
    (bind _asbp_iss_test_character (cast `/Game/InfluenceSpawnSystem/Blueprints/ISSTestSystems/BP_ISS_TestCharacter` (`self.K2_GetPawn`)))
    (`/Game/InfluenceSpawnSystem/Blueprints/ISSTestSystems/BP_ISS_TestCharacter.ServerTestDeath` _asbp_iss_test_character)))

(event `RespawnPlayerCharacter`
  (params (`Player Controller` :type "PlayerController Object Reference") (ControllerOnRespawn :type "Controller Object Reference"))
  ;[1 1 1] TEST RESPAWN
  ;;[1 1 1] RespawnPlayerCharacter
  (bind _asbp_iss_test_game_mode (cast `/Game/InfluenceSpawnSystem/Blueprints/ISSTestSystems/BP_ISS_TestGameMode` (`GameplayStatics.GetGameMode`)))
  (`/Game/InfluenceSpawnSystem/Blueprints/ISSTestSystems/BP_ISS_TestGameMode.CharacterRespawn` _asbp_iss_test_game_mode `Player Controller` ControllerOnRespawn))

(fn `UserConstructionScript`)
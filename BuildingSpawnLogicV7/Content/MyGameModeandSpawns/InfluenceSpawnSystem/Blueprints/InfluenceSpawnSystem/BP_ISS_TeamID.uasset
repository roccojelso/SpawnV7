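; Component that tags its owning actor with a team ID for the Influence Spawn System, with plain get and set functions.
; ServerInitializeTeam stores the team, multicasts it and opens a Tick gate.
; The gated Tick uses a delay to periodically check the game mode's BP_ISS_InfluenceSpawnSystem debug flag.
; When enabled, it draws the team name at the owner's location, color-coded by team.
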(event `DrawDebugTeamType`
  (params (TextLocation :type "Vector Structure") (Text :type String) (Selection :type "/Game/MyGameModeandSpawns/InfluenceSpawnSystem/Blueprints/InfluenceSpawnSystem/Data/ENUM_ISS_TeamType Enum" :default "NewEnumerator0"))
  ;[1 1 1] EVENT TICK
  ;;[1 1 1] DrawDebugTeamType
  (switch `/Game/MyGameModeandSpawns/InfluenceSpawnSystem/Blueprints/InfluenceSpawnSystem/Data/ENUM_ISS_TeamType` Selection
    (:`NewEnumerator0`
      (`KismetSystemLibrary.DrawDebugString` TextLocation Text null (struct :`R` 1.0 :`G` 1.0 :`B` 1.0 :`A` 1.0) 1.2))
    (:`NewEnumerator1`
      (`KismetSystemLibrary.DrawDebugString` TextLocation Text null (struct :`R` 1.0 :`B` 0.012991 :`A` 1.0) 1.2))
    (:`NewEnumerator2`
      (`KismetSystemLibrary.DrawDebugString` TextLocation Text null (struct :`G` 0.097639 :`B` 1.0 :`A` 1.0) 1.2))))

(event `self.ReceiveTick`
  (params (DeltaSeconds :type "Float (single-precision)"))
  (bind _returnvalue (`Actor.GetComponentByClass` (`GameplayStatics.GetGameMode`) "/Game/MyGameModeandSpawns/InfluenceSpawnSystem/Blueprints/InfluenceSpawnSystem/BP_ISS_InfluenceSpawnSystem.BP_ISS_InfluenceSpawnSystem_C"))
  ;[1 1 1] EVENT TICK
  ;;[1 1 1] Unlock gate for server only
  (`/Engine/EditorBlueprintResources/StandardMacros.Gate` true :!label _label
    (:`Exit`
      (`KismetSystemLibrary.Delay` 1.2)
      ;;[1 1 1] Condition
      (`/Engine/EditorBlueprintResources/StandardMacros.IsValid` _returnvalue
        (:`Is Valid`
          (if (`/Game/MyGameModeandSpawns/InfluenceSpawnSystem/Blueprints/InfluenceSpawnSystem/BP_ISS_InfluenceSpawnSystem.Debug Draw Character Identification` _returnvalue)
            ;;[1 1 1] DrawDebugTeamType
            (`self.DrawDebugTeamType` (`Actor.K2_GetActorLocation` (`self.GetOwner`)) (`|GetEnumeratorNameAsString` (`self.Team`)) (`self.Team`))))))))

(event `UnlockEventTick`
  ;[1 1 1] EVENT TICK
  ;;[1 1 1] Unlock gate for server only
  ;;;[1 1 1] UnlockEventTick
  (goto _label :!via `Open`))

(event `ServerInitializeTeam`
  (params (Team :type "/Game/MyGameModeandSpawns/InfluenceSpawnSystem/Blueprints/InfluenceSpawnSystem/Data/ENUM_ISS_TeamType Enum" :default "NewEnumerator0"))
  ;[1 1 1] Initialize Character Identificator
  (bind _output_get (set `self.Team` Team))
  (`self.MulticastInitializeTeam` _output_get)
  (`self.UnlockEventTick`))

(event `MulticastInitializeTeam`
  (params (Team :type "/Game/MyGameModeandSpawns/InfluenceSpawnSystem/Blueprints/InfluenceSpawnSystem/Data/ENUM_ISS_TeamType Enum" :default "NewEnumerator0"))
  ;[1 1 1] Initialize Character Identificator
  (set `self.Team` Team))

(fn `GetTeam`
  (returns (Team :type "/Game/MyGameModeandSpawns/InfluenceSpawnSystem/Blueprints/InfluenceSpawnSystem/Data/ENUM_ISS_TeamType Enum"))
  (return (`self.Team`)))

(fn `SetTeam`
  (params (Team :type "/Game/MyGameModeandSpawns/InfluenceSpawnSystem/Blueprints/InfluenceSpawnSystem/Data/ENUM_ISS_TeamType Enum" :default "NewEnumerator0"))
  (set `self.Team` Team))